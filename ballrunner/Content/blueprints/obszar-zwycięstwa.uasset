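; Victory area actor that ends the level when the player pawn overlaps its box trigger.
; If any Cone_bp_1 actors (the crystals) remain, it only prints a Polish reminder to collect them.
; Otherwise CompleteLvl opens the entry following the current level's name in the LvlNames array.
; IsFinalLvl always returns false because its last-index comparison is unconnected, so the quit-game branch never runs.
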(event `self.Box.OnComponentBeginOverlap`
  (params (OverlappedComponent :type "PrimitiveComponent Object Reference") (OtherActor :type "Actor Object Reference") (OtherComp :type "PrimitiveComponent Object Reference") (OtherBodyIndex :type Integer) (bFromSweep :type Boolean) (SweepResult :type "HitResult Structure (by ref)"))
  (if (== OtherActor (`GameplayStatics.GetPlayerPawn` 0))
    (bind _outactors (`GameplayStatics.GetAllActorsOfClass` "/Game/blueprints/collectable/cone_bp_1.cone_bp_1_C"))
    (if (> (`KismetArrayLibrary.Array_Length` _outactors) 0)
      (`KismetSystemLibrary.PrintString` "zostały ci kryształy do zebrania")
      (else
        (`self.complete lvl`)))))

(fn `complete lvl`
  (if (`self.is final lvl`)
    (`KismetSystemLibrary.QuitGame` null "Quit")
    (else
      (`self.load next lvl`))))

(fn `get current lvl index`
  (returns (`return node` :type Integer))
  (bind _returnvalue (`GameplayStatics.GetCurrentLevelName` true))
  (return (`KismetArrayLibrary.Array_Find` (`self.lvl names`) _returnvalue)))

(fn `get next lvl name`
  (returns (output :type String))
  (return (`|GetArrayItem` (`self.lvl names`) (+ (`self.get current lvl index`) 1))))

(fn `is final lvl`
  (returns (`return value` :type Boolean))
  (return false))

(fn `load next lvl`
  (`GameplayStatics.OpenLevel` (`KismetStringLibrary.Conv_StringToName` (`self.get next lvl name`))))

(fn `UserConstructionScript`)