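; Crystal collectable Blueprint that is drawn into the player and vanishes when picked up.
; When the player pawn overlaps Trigger1, a timeline moves the crystal toward the pawn's current location while shrinking it and fading its point light.
; Each update lerps from the actor's current location and scale, so the motion compounds.
; When the timeline finishes, it plays a 2D sound and destroys the actor after a short delay.
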(event `self.trigger1.OnComponentBeginOverlap`
  (params (OverlappedComponent :type "PrimitiveComponent Object Reference") (OtherActor :type "Actor Object Reference") (OtherComp :type "PrimitiveComponent Object Reference") (OtherBodyIndex :type Integer) (bFromSweep :type Boolean) (SweepResult :type "HitResult Structure (by ref)"))
  (if (== OtherActor (`GameplayStatics.GetPlayerPawn` 0))
    (bind (_direction _crystal_location _scale _light) (`Timeline|Timeline_0`)
      (:`Update`
        (`self.K2_SetActorLocation` (`KismetMathLibrary.VLerp` (`self.K2_GetActorLocation`) (`self.K2_GetActorLocation` (`GameplayStatics.GetPlayerPawn` 0)) _crystal_location) true)
        (`self.SetActorScale3D` (`KismetMathLibrary.VLerp` (`self.GetActorScale3D`) (0.0 0.0 0.0) _scale))
        (`LightComponent.SetIntensity` (`self.PointLight`) (`KismetMathLibrary.Lerp` 100.0 0.0 _light)))
      (:`Finished`
        (`GameplayStatics.SpawnSound2D` "/Game/blueprints/93166__sandyrb__coke-cans-crush-c617-002.93166__sandyrb__coke-cans-crush-c617-002" 1.0 1.0 0.0 null)
        (`KismetSystemLibrary.Delay` 0.2)
        (`self.K2_DestroyActor`)))))

(fn `UserConstructionScript`)